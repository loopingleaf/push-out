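; Actor component that temporarily stuns the player pawn that owns it.
; Its Stun event compares the owner's display name against four hardcoded player Blueprint names, BPPlayer1 through BPPlayer4, then casts to the matching class.
; It sets that player's IsPlayerStun flag, waits three seconds and clears it, repeating the same logic in each branch rather than using a shared base class or interface.
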(event EventStun
  (params (isStun :type Boolean))
  (bind _returnvalue (Components|GetOwner))
  (bind _returnvalue_2 (Utilities|GetDisplayName _returnvalue))
  (if (Utilities|Enum|Equal(Enum) _returnvalue_2 "BPPlayer1")
    (bind _asbpplayer_1 (Utilities|Casting|CastToBPPlayer1 _returnvalue))
    (Variables|/Game/Blueprints/BP_Player.BP_Player_C|SetisPlayerStun _asbpplayer_1 true)
    (Utilities|FlowControl|Delay 3.0)
    (Variables|/Game/Blueprints/BP_Player.BP_Player_C|SetisPlayerStun _asbpplayer_1 false)
    (elif (Utilities|Enum|Equal(Enum) _returnvalue_2 "BPPlayer2")
      (bind _asbpplayer_2 (Utilities|Casting|CastToBPPlayer2 _returnvalue))
      (Variables|/Game/Blueprints/BP_Player.BP_Player_C|SetisPlayerStun _asbpplayer_2 true)
      (Utilities|FlowControl|Delay 3.0)
      (Variables|/Game/Blueprints/BP_Player.BP_Player_C|SetisPlayerStun _asbpplayer_2 false)
      (elif (Utilities|Enum|Equal(Enum) _returnvalue_2 "BPPlayer3")
        (bind _asbpplayer_3 (Utilities|Casting|CastToBPPlayer3 _returnvalue))
        (Variables|/Game/Blueprints/BP_Player.BP_Player_C|SetisPlayerStun _asbpplayer_3 true)
        (Utilities|FlowControl|Delay 3.0)
        (Variables|/Game/Blueprints/BP_Player.BP_Player_C|SetisPlayerStun _asbpplayer_3 false)
        (elif (Utilities|Enum|Equal(Enum) _returnvalue_2 "BPPlayer4")
          (bind _asbpplayer_4 (Utilities|Casting|CastToBPPlayer4 _returnvalue))
          (Variables|/Game/Blueprints/BP_Player.BP_Player_C|SetisPlayerStun _asbpplayer_4 true)
          (Utilities|FlowControl|Delay 3.0)
          (Variables|/Game/Blueprints/BP_Player.BP_Player_C|SetisPlayerStun _asbpplayer_4 false))))))