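; Component that makes its owning actor slide when pushed, with weight controlling how quickly it stops.
; The Pushed event stores direction, speed and weight, then Tick moves the owner with a swept SetActorLocation.
; Each frame subtracts elapsed push time times weight from speed until it stops; this decay is not delta-scaled, so it depends on frame rate.
; Disconnected leftover nodes hold a line-trace push setup and a copy of the movement logic.
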(event EventTick
  (params (DeltaSeconds :type Float%20%28single-precision%29))
  (bind _returnvalue (Components|GetOwner))
  (if (Variables|Default|GetisMoving)
    (Variables|Default|SetmovingFor (+ DeltaSeconds (Variables|Default|GetmovingFor)))
    (Variables|Default|Setspeed (Math|Float|Max(Float) (- (Variables|Default|Getspeed) (* (Variables|Default|GetmovingFor) (Variables|Default|Getweight))) 0.0))
    (if (<= (Variables|Default|Getspeed) 0.0001)
      (Variables|Default|SetisMoving false)
      (else
        (Transformation|SetActorLocation _returnvalue (+ (Transformation|GetActorLocation _returnvalue) (* (Variables|Default|Getdirection) (* (Variables|Default|Getspeed) DeltaSeconds))) true false)))
    (else
      (Variables|Default|Setspeed 0.0)
      (Variables|Default|SetmovingFor 0.0))))

(event EventPushed
  (params (Direction :type Vector :default "0, 0, 0") (Speed :type Float%20%28single-precision%29) (Weight :type Float%20%28single-precision%29))
  (Variables|Default|SetisMoving true)
  (Variables|Default|Setdirection Direction)
  (Variables|Default|Setspeed Speed)
  (Variables|Default|Setweight Weight))