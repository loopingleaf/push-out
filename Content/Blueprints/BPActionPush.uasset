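; BPActionPush is a component-style Blueprint that lets its owner push objects in front of it.
; On press, PushAction line-traces on the Visibility channel along the owner's forward vector up to Range, with persistent debug drawing.
; Hit actors implementing IPushable receive PushMessage with Force and an unnormalized direction from impact location to actor location.
; IsPushActionPressed and IsPushing track input and push state.
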(event EventBeginPlay)

(event EventTick
  (params (DeltaSeconds :type Float%20%28single-precision%29)))

(fn PushAction
  (params (isActionPressed :type Boolean))
  (bind _returnvalue (Components|GetOwner))
  (if isActionPressed
    (Variables|Default|SetisPushActionPressed true)
    (Variables|Default|SetisPushing true)
    (bind _outhit (Collision|LineTraceByChannel (Transformation|GetActorLocation (Components|GetOwner)) (+ (Transformation|GetActorLocation _returnvalue) (* (Math|Vector|GetForwardVector (Transformation|GetActorRotation _returnvalue)) (Variables|Default|Getrange))) "TraceTypeQuery1" false 0 "Persistent"))
    (if (Utilities|DoesObjectImplementInterface (.hitactor _outhit) "/Game/IPushable.IPushable_C")
      (Class|IPushable|Push(Message) (.hitactor _outhit) (- (Transformation|GetActorLocation (.hitactor _outhit)) (.location _outhit)) (Variables|Default|Getforce))
      (Variables|Default|SetisPushing false)
      (else
        (Variables|Default|SetisPushing false)))
    (elif (not (Variables|Default|GetisPushing))
      (Variables|Default|SetisPushActionPressed false))))