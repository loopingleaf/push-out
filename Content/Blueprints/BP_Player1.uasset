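; BP_Player1 is a player pawn that moves from externally supplied input and respawns when it falls out of the level.
; Its Multiplayer event takes a value and a type string, turning "Forward" or "Right" into movement input along fixed world X or Y axes.
; BeginPlay stores the starting location, and Tick teleports the actor back there once it drops below a fixed height.
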(event EventMultiplayer
  (params (Value :type Float%20%28single-precision%29) (Type :type String))
  ;[1 1 1] Execute input
  (if (Utilities|Enum|Equal(Enum) Type "Forward")
    (Pawn|Input|AddMovementInput "1.000000, 0, 0" Value false)
    (elif (Utilities|Enum|Equal(Enum) Type "Right")
      (Pawn|Input|AddMovementInput "0,1.000000, 0" Value false))))

(event EventHit)

(event EventBeginPlay
  (Variables|Default|SetinitialPos (Transformation|GetActorLocation)))

(event EventTick
  (params (DeltaSeconds :type Float%20%28single-precision%29))
  (if (< (.z (Transformation|GetActorLocation)) -8e+02)
    (Transformation|SetActorLocation (Variables|Default|GetinitialPos) false true)))

(fn ConstructionScript)