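; BP_Player is a player character that moves along fixed world axes, can be stunned and respawns after falling.
; Its Multiplayer event receives named Forward or Right axis values and applies movement input unless the player is stunned.
; Capsule overlaps are forwarded to BPPlayer's Hit, and Stun calls are delegated to BPStun.
; Tick teleports the player back to its BeginPlay location when it drops below a height threshold.
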(event OnComponentBeginOverlap(CapsuleComponent)
  (params (OverlappedComponent :type Primitive%20Component%20Object%20Reference) (OtherActor :type Actor%20Object%20Reference) (OtherComp :type Primitive%20Component%20Object%20Reference) (OtherBodyIndex :type Integer) (bFromSweep :type Boolean) (SweepResult :type Hit%20Result%20Structure%20%28by%20ref%29))
  (Default|Hit (Variables|Default|GetBPPlayer) OtherActor))

(event EventMultiplayer
  (params (Value :type Float%20%28single-precision%29) (Type :type String))
  ;[1 1 1] Execute input
  (if (not (Variables|Default|GetisPlayerStun))
    (if (Utilities|Enum|Equal(Enum) Type "Forward")
      (Pawn|Input|AddMovementInput "1.000000, 0, 0" Value false)
      (elif (Utilities|Enum|Equal(Enum) Type "Right")
        (Pawn|Input|AddMovementInput "0,1.000000, 0" Value false)))))

(event EventBeginPlay
  (Variables|Default|SetinitialPos (Transformation|GetActorLocation)))

(event EventTick
  (params (DeltaSeconds :type Float%20%28single-precision%29))
  (if (< (.z (Transformation|GetActorLocation)) -8e+02)
    (Transformation|SetActorLocation (Variables|Default|GetinitialPos) false true)))

(event EventStun
  (params (isStun :type Boolean))
  (Default|Stun (Variables|Default|GetBP_Stun) isStun))

(fn ConstructionScript)